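; BP_RocksSource is a rock emitter actor that repeatedly spawns BP_Projectile actors from a box-shaped area.
; Tick feeds a three-second latent Delay, so a spawn fires roughly every three seconds rather than every frame.
; Each projectile appears at a random point within the SpawnRocks box, facing along the Arrow component's forward vector.
; BeginPlay enables input from the first player controller, though the graph handles no input events.
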(event EventBeginPlay
  (Input|EnableInput (Game|GetPlayerController 0)))

(event Collision|EventActorBeginOverlap
  (params (OtherActor :type Actor%20Object%20Reference)))

(event EventTick
  (params (DeltaSeconds :type Float%20%28single-precision%29))
  (bind _spawnrocks (Variables|Default|GetSpawnRocks))
  (Utilities|FlowControl|Delay 3.0)
  (Game|SpawnActorfromClass "/Game/Astronaut/Rocks/BP_Projectile.BP_Projectile_C" (Math|Transform|MakeTransform (Math|Random|RandomPointinBoundingBox (Transformation|GetWorldLocation _spawnrocks) (Components|Box|GetScaledBoxExtent _spawnrocks)) (Math|Rotator|MakeRotfromX (Math|Vector|GetForwardVector (Transformation|GetWorldRotation (Variables|Default|GetArrow)))) "1,1,1") "Undefined" 0 0))

(fn ConstructionScript)