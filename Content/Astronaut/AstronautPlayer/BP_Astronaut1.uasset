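; BP_Astronaut1 is a physics-driven player astronaut that rolls on the MoveRight axis and thrusts along its arrow with left-click impulses.
; Both inputs trigger left/right pump events that briefly fire particles and sound, gated by DoOnce.
; A Delay on Tick drains oxygen about every three seconds, while Damage reduces health.
; Depleting either calls Dead, which notifies BP_GameMode of the player's death.
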(event Custom|LeftPump
  (bind _leftparticles (Variables|Default|GetLeftParticles))
  ;[1 1 1] Right/Left Particles pump
  (Components|Activation|Activate _leftparticles false)
  (Utilities|FlowControl|DoOnce false :!label _label
    (:Completed
      (Audio|PlaySoundatLocation "/Game/Astronaut/AstronautPlayer/Smoke01_Cue.Smoke01_Cue" (Transformation|GetWorldLocation _leftparticles) "0, 0, 0" 1.0 1.0 0.0 0 0 0)
      (Utilities|FlowControl|Delay 0.2)
      (Components|Activation|Deactivate _leftparticles)
      (goto _label Reset))))

(event Custom|RightPump
  (bind _rightparticles (Variables|Default|GetRightParticles))
  ;[1 1 1] Right/Left Particles pump
  (Components|Activation|Activate _rightparticles false)
  (Utilities|FlowControl|DoOnce false :!label _label
    (:Completed
      (Audio|PlaySoundatLocation "/Game/Astronaut/AstronautPlayer/Smoke01_Cue.Smoke01_Cue" (Transformation|GetWorldLocation _rightparticles) "0, 0, 0" 1.0 1.0 0.0 0 0 0)
      (Utilities|FlowControl|Delay 0.2)
      (Components|Activation|Deactivate _rightparticles)
      (goto _label Reset))))

(event EventBeginPlay
  (Input|EnableInput (Game|GetPlayerController 0)))

(event EventTick
  (params (DeltaSeconds :type Float%20%28single-precision%29))
  (Utilities|FlowControl|Delay 3.0)
  (Variables|Default|Setoxigen (- (Variables|Default|Getoxigen) 5.0))
  (if (<= (Variables|Default|Getoxigen) 0.0)
    (CallFunction|Dead)))

(event Input|AxisEvents|InputAxisMoveRight
  (params (AxisValue :type Float%20%28single-precision%29))
  ;[1 1 1] Roll left/right
  (Transformation|AddWorldRotation (Variables|Default|GetPhysicsBox) (Math|Rotator|MakeRotator AxisValue 0.0 0.0) false false)
  (if (> AxisValue 0.0)
    (CallFunction|LeftPump)
    (elif (< AxisValue 0.0)
      (CallFunction|RightPump))))

(event Input|MouseEvents|LeftMouseButton
  (params (Key :type Key%20Structure :default "None"))
  (:Pressed
    (Physics|AddImpulse (Variables|Default|GetPhysicsBox) (* (Math|Rotator|GetRotationXVector (Transformation|GetWorldRotation (Variables|Default|GetArrow))) (Variables|Default|GetImpulseValue)) "None" false)
    (CallFunction|LeftPump)
    (CallFunction|RightPump)))

(event Input|MouseEvents|RightMouseButton
  (params (Key :type Key%20Structure :default "None")))

(fn ConstructionScript)

(fn Damage
  (Variables|Default|SetFullHealth (- (Variables|Default|GetFullHealth) 15.0))
  (if (< (Variables|Default|GetFullHealth) 1.0)
    (CallFunction|Dead)))

(fn Dead
  (bind _asbp_game_mode (Utilities|Casting|CastToBP_GameMode (Game|GetGameMode)))
  (Default|NotifyPlayerDead _asbp_game_mode))