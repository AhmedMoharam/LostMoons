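; BP_Projectile is a projectile actor, stored with the rock assets, that damages the astronaut on overlap.
; When its sphere collision overlaps a BP_Astronaut1, it prints a debug "Hello", calls that astronaut's Damage function and destroys itself.
; A separate actor-level overlap sends standard ApplyDamage to player pawn 0 using its Damage variable, so one contact can trigger both damage paths.
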(event OnComponentBeginOverlap(SphereCollision)
  (params (OverlappedComponent :type Primitive%20Component%20Object%20Reference) (OtherActor :type Actor%20Object%20Reference) (OtherComp :type Primitive%20Component%20Object%20Reference) (OtherBodyIndex :type Integer) (bFromSweep :type Boolean) (SweepResult :type Hit%20Result%20Structure%20%28by%20ref%29))
  (bind _asbp_astronaut_1 (Utilities|Casting|CastToBP_Astronaut1 OtherActor))
  (Development|PrintString "Hello")
  (Default|Damage _asbp_astronaut_1)
  (Actor|DestroyActor))

(event EventBeginPlay)

(event Collision|EventActorBeginOverlap
  (params (OtherActor :type Actor%20Object%20Reference))
  (if (== OtherActor (Game|Player|GetPlayerPawn 0))
    (Game|Damage|ApplyDamage OtherActor (Variables|Default|GetDamage) 0 self)))

(fn ConstructionScript)